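; BP_Character is the player pawn for the Factions game, with yaw-relative movement, look input and right-mouse aiming.
; On BeginPlay, the local player pushes and displays the Supply Raid HUD, while other copies print their team comparison against the first player state.
; Right mouse toggles the character state between Aiming and Default.
; Each locally controlled tick eases the radar's physical radius toward a state-based target, narrowing it while aiming.
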(event `self.ReceiveBeginPlay`
  (bind _returnvalue (pcsubsystem `UserInterfaceSubsystem` (`GameplayStatics.GetPlayerController` 0)))
  (`|ExecutionSequence`
    (:`then_0`
      (if (`self.IsLocallyControlled`)
        (bind _returnvalue_2 (`UserInterfaceSubsystem.PushHUD` _returnvalue "/Game/Factions/UserInterface/HUD/WBP_HUD_SupplyRaid.WBP_HUD_SupplyRaid_C"))
        (`UserInterfaceSubsystem.DisplayHUD` _returnvalue _returnvalue_2)
        (else
          (bind _returnvalue_3 (`FactionsSessionSubsystem.CompareTeams` (subsystem `FactionsSessionSubsystem`) self (`GameplayStatics.GetPlayerState` 0)))
          (`KismetSystemLibrary.PrintString` (`|GetEnumeratorNameAsString` _returnvalue_3)))))))

(event `Key|RightMouseButton`
  (params (Key :type "Key Structure"))
  (:`Pressed`
    (`self.SetCharacterState` "Aiming"))
  (:`Released`
    (`self.SetCharacterState` "Default")))

(event `self.ReceiveTick`
  (params (DeltaSeconds :type "Float (single-precision)"))
  (if (`self.IsLocallyControlled`)
    (`RadarSubsystem.SetPhysicalRadius` (`self.RadarSubsystem`) (`KismetMathLibrary.FInterpTo` (`RadarSubsystem.PhysicalRadius` (`self.RadarSubsystem`)) (select `ECharacterState` (`self.CharacterState`) :`Default` 1500.0 :`Aiming` 500.0 :`Down` 1500.0 :`Backpack` 1500.0) DeltaSeconds 2.0))))

(event `InputAxis|MoveForward`
  (params (AxisValue :type "Float (single-precision)"))
  (bind (_returnvalue_roll _returnvalue_pitch _returnvalue_yaw) (`KismetMathLibrary.BreakRotator` (`self.GetControlRotation`)))
  (`self.AddMovementInput` (`KismetMathLibrary.GetForwardVector` (`KismetMathLibrary.MakeRotator` 0.0 0.0 _returnvalue_yaw)) AxisValue))

(event `InputAxis|MoveRight`
  (params (AxisValue :type "Float (single-precision)"))
  (bind (_returnvalue_roll _returnvalue_pitch _returnvalue_yaw) (`KismetMathLibrary.BreakRotator` (`self.GetControlRotation`)))
  (`self.AddMovementInput` (`KismetMathLibrary.GetRightVector` (`KismetMathLibrary.MakeRotator` 0.0 0.0 _returnvalue_yaw)) AxisValue))

(event `InputAxis|LookUp`
  (params (AxisValue :type "Float (single-precision)"))
  (`self.AddControllerPitchInput` AxisValue))

(event `InputAxis|LookRight`
  (params (AxisValue :type "Float (single-precision)"))
  (`self.AddControllerYawInput` AxisValue))

(fn `UserConstructionScript`)